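; BP_AudioManager swaps the game's audio for a stinger and tension music when a wanted or innocent target is killed.
; On BeginPlay it binds both kill delegates of SplitScreenGameMode to one handler.
; The handler stops the Audio component, plays one of ten random 2D sounds, then starts tension music after a short delay.
; A longer delay then restarts the Audio component from the beginning.
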(event `self.ReceiveBeginPlay`
  (bind _assplit_screen_game_mode (cast `/Game/Salvo/SplitScreenGameMode` (`GameplayStatics.GetGameMode`)))
  (add `/Game/Salvo/SplitScreenGameMode.OnWantedKilled` _assplit_screen_game_mode (delegate `OnWantedKilled_Event`))
  (add `/Game/Salvo/SplitScreenGameMode.OnInnocentKilled` _assplit_screen_game_mode (delegate `OnWantedKilled_Event`)))

(event `OnWantedKilled_Event`
  (params (ID :type Integer))
  (`AudioComponent.Stop` (`self.Audio`))
  (`GameplayStatics.PlaySound2D` (`KismetArrayLibrary.Array_Random` (`|MakeArray` "/Game/Sounds/Screams/s1.s1" "/Game/Sounds/Screams/s2.s2" "/Game/Sounds/Screams/s3.s3" "/Game/Sounds/Screams/s4.s4" "/Game/Sounds/Screams/s5.s5" "/Game/Sounds/Screams/s6.s6" "/Game/Sounds/Screams/s7.s7" "/Game/Sounds/Screams/s8.s8" "/Game/Sounds/Screams/s9.s9" "/Game/Sounds/Screams/s10.s10" :!type "SoundBase Object Reference")) 1.5 1.0 0.0 null null)
  (`KismetSystemLibrary.Delay` 1.0)
  (`GameplayStatics.PlaySound2D` "/Game/Sounds/tensionmusic.tensionmusic" 0.9 1.0 0.0 null null)
  (`KismetSystemLibrary.Delay` 14.0)
  (`AudioComponent.Play` (`self.Audio`) 0.0))

(fn `UserConstructionScript`)